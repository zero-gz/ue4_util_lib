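; Utility Blueprint with helper functions for oscillating yaw rotation and cursor picking.
; ActorRotateZ swings a scene component by a speed scaled with delta time, flipping a by-reference sign flag when relative yaw from GetZAngle reaches either symmetric angle limit.
; GetCursorActor traces under player 0's cursor on a given channel and returns the hit actor and location when something is hit.
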(fn `actor_rotate_z`
  (params (scene_comp :type "SceneComponent Object Reference") (delta_time :type "Float (double-precision)" :default 0.0) (abs_angle :type "Float (double-precision)" :default 360.0) (speed :type "Float (double-precision)" :default 10.0) (sign :type "Boolean (by ref)"))
  (bind _z_angle (`self.get_z_angle` scene_comp))
  (`|ExecutionSequence`
    (:`then_0`
      (if (or (<= _z_angle (* abs_angle -1.0)) (>= _z_angle abs_angle))
        (`|VariableSetRef` sign (not sign))))
    (:`then_1`
      (`SceneComponent.K2_AddLocalRotation` scene_comp (`KismetMathLibrary.MakeRotator` 0.0 0.0 (* delta_time speed (select `bool` sign :`false` 1.0 :`true` -1.0 :!type "Float (single-precision)"))) false false))))

(fn `get_cursor_actor`
  (params (channel :type "ETraceTypeQuery Enum" :default "TraceTypeQuery1"))
  (returns (hit_actor :type "Actor Object Reference") (hit_location :type "Vector Structure"))
  (bind (_hitresult _returnvalue) (`PlayerController.GetHitResultUnderCursorByChannel` (`GameplayStatics.GetPlayerController` "0") channel false))
  (bind (_bblockinghit _binitialoverlap _time _distance _location _impactpoint _normal _impactnormal _physmat _hitactor) (`GameplayStatics.BreakHitResult` _hitresult))
  (if _returnvalue
    (return _hitactor _location)))

(fn `get_z_angle`
  (params (scene_comp :type "SceneComponent Object Reference"))
  (returns (z_angle :type "Float (double-precision)"))
  (return (.yaw (`SceneComponent.RelativeRotation` scene_comp))))